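; BP_ProjectileBase is a base homing projectile Blueprint for the Inviturrets game that carries damage to a target.
; Each tick it moves its root toward the target's current location at constant speed using VInterpToConstant, without sweeping or collision checks.
; On reaching the target's position within a small tolerance it sends a damage message and destroys itself.
; It also destroys itself if the target is no longer valid.
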(event EventBeginPlay)

(event Collision|EventActorBeginOverlap
  (params (OtherActor :type Actor%20Object%20Reference)))

(event EventTick
  (params (DeltaSeconds :type Float%20%28single-precision%29))
  (bind _returnvalue (Transformation|GetActorLocation))
  (bind _target (Variables|Default|GetTarget)
    (:then
      (if (Utilities|Operators|EqualEqual _returnvalue (Transformation|GetActorLocation _target) 1.0)
        (Class|IDamagable|DoDamage(Message) (Variables|Default|GetTarget) (Variables|Default|GetDamage))
        (Actor|DestroyActor)
        (else
          (Transformation|SetWorldLocation (Variables|Default|GetDefaultSceneRoot) (Math|Interpolation|VInterptoConstant _returnvalue (Transformation|GetActorLocation _target) DeltaSeconds (Variables|Default|GetProjectileSpeed)) false false))))
    (:else
      (Actor|DestroyActor))))

(fn ConstructionScript)