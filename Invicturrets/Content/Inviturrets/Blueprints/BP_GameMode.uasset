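; Tower-defense game mode for Inviturrets that tracks enemy kills against the level data asset's enemy count and resolves wins and losses.
; Each kill fires a dispatcher, and reaching the count opens the data asset's next level, if valid, while defeat opens the menu.
; BeginPlay only calls the parent.
; Blueprint logic for HUD caching, music and timed waypoint spawning is disconnected and never runs.
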(event Custom|SpawnEnemy)

(event EventBeginPlay
  (|CallParentFunction))

(fn ConstructionScript)

(fn EnemyKilledBP
  (bind _result (Math|Integer|IncrementInt (Variables|Default|GetKillCount_0))
    (:%20%20
      (Default|CallEnemyKilledDispatcher _result)
      (if (>= _result (Variables|/Game/Inviturrets/Blueprints/DPA_LevelData.DPA_LevelData_C|GetEnemyCount (Variables|Default|GetLevelDataAsset)))
        (CallFunction|GameWonBP)))))

(fn GameWonBP
  (Development|PrintString "Youn won!")
  (Utilities|Time|ClearandInvalidateTimerbyHandle (Variables|Default|GetSpawTimerHandle))
  (bind _nextlevel (Variables|/Game/Inviturrets/Blueprints/DPA_LevelData.DPA_LevelData_C|GetNextLevel (Variables|Default|GetLevelDataAsset))
    (:then
      (Game|OpenLevel(byObjectReference) _nextlevel))
    (:else)))

(fn GameOverVP
  (Development|PrintString "You lost")
  (Utilities|Time|ClearandInvalidateTimerbyHandle (Variables|Default|GetSpawTimerHandle))
  (Game|OpenLevel(byObjectReference) "/Game/Inviturrets/Levels/Menu.Menu"))

(fn GetLevelsEnemyCountBP
  (return (Variables|/Game/Inviturrets/Blueprints/DPA_LevelData.DPA_LevelData_C|GetEnemyCount (Variables|Default|GetLevelDataAsset))))