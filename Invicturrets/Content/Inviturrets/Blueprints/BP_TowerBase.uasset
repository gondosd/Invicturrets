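; BP_TowerBase is a turret tower that targets and fires at BP_EnemyBase actors within a sphere sized to its Range in construction.
; A looping timer is set at ShootFrequency, and Shoot picks the closest overlapping enemy as the active target.
; Tick interpolates RotationRoot's yaw toward that target.
; Once aligned, Tick spawns a BP_ProjectileBase at FireLoc with the target passed in, then clears the target and closest distance.
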(event Custom|Shoot
  (for _array_element (Collision|GetOverlappingActors (Variables|Default|GetSphere) "/Game/Inviturrets/Blueprints/BP_EnemyBase.BP_EnemyBase_C" :!class /Script/Engine.PrimitiveComponent)
    (if (<= (Transformation|GetDistanceTo _array_element) (Variables|Default|GetClosestDistance))
      (Variables|Default|SetClosestDistance (Transformation|GetDistanceTo _array_element))
      (Variables|Default|SetActiveTargetPointer _array_element))))

(event EventBeginPlay
  (Utilities|Time|SetTimerbyEvent (EventDispatchers|CreateEvent :!event Custom|Shoot) (Variables|Default|GetShootFrequency) true))

(event EventTick
  (params (DeltaSeconds :type Float%20%28single-precision%29))
  (bind _rotationroot (Variables|Default|GetRotationRoot))
  (bind _relativerotation (Variables|/Script/Engine.SceneComponent|GetRelativeRotation _rotationroot))
  (Variables|Default|GetActiveTargetPointer
    (:then
      (if (Utilities|Operators|EqualEqual _relativerotation (Math|Rotator|MakeRotator 0.0 0.0 (.yaw (Math|Rotator|FindLookatRotation (Transformation|GetWorldLocation (Variables|Default|GetRotationRoot)) (Transformation|GetWorldLocation (Variables|/Script/Engine.Actor|GetRootComponent (Variables|Default|GetActiveTargetPointer)))))) 1.0)
        (bind _activetargetpointer (Variables|Default|GetActiveTargetPointer)
          (:then
            (Game|SpawnActorfromClass "/Game/Inviturrets/Blueprints/BP_ProjectileBase.BP_ProjectileBase_C" (Transformation|GetWorldTransform (Variables|Default|GetFireLoc)) "Undefined" 0 _activetargetpointer 0)
            (Variables|Default|SetClosestDistance 1e+08)
            (Variables|Default|SetActiveTargetPointer 0))
          (:else))
        (else
          (Transformation|SetRelativeRotation (Variables|Default|GetRotationRoot) (Math|Interpolation|RInterpTo _relativerotation (Math|Rotator|MakeRotator 0.0 0.0 (.yaw (Math|Rotator|FindLookatRotation (Transformation|GetWorldLocation (Variables|Default|GetRotationRoot)) (Transformation|GetWorldLocation (Variables|/Script/Engine.Actor|GetRootComponent (Variables|Default|GetActiveTargetPointer)))))) DeltaSeconds (Variables|Default|GetTurretRotationSpeed)) false false))))
    (:else)))

(fn ConstructionScript
  (Components|Sphere|SetSphereRadius (Variables|Default|GetSphere) (Variables|Default|GetRange) true))